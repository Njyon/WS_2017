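; Decorative bird prop Blueprint that plays a looping flight animation on a group of skeletal mesh birds.
; On BeginPlay it starts the same fly loop on the meshes in three batches, separated by short delays so the wingbeats can fall out of sync.
; A final delay leads to nothing, and the graph contains no movement logic.
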(event `self.ReceiveBeginPlay`
  (`SkeletalMeshComponent.PlayAnimation` (`self.Bird`) "/Game/Characters/prop_bird/anim_propBird_flyLoop.anim_propBird_flyLoop" true)
  (`SkeletalMeshComponent.PlayAnimation` (`self.SkeletalMesh7`) "/Game/Characters/prop_bird/anim_propBird_flyLoop.anim_propBird_flyLoop" true)
  (`SkeletalMeshComponent.PlayAnimation` (`self.SkeletalMesh`) "/Game/Characters/prop_bird/anim_propBird_flyLoop.anim_propBird_flyLoop" true)
  (`SkeletalMeshComponent.PlayAnimation` (`self.SkeletalMesh1`) "/Game/Characters/prop_bird/anim_propBird_flyLoop.anim_propBird_flyLoop" true)
  (`SkeletalMeshComponent.PlayAnimation` (`self.SkeletalMesh2`) "/Game/Characters/prop_bird/anim_propBird_flyLoop.anim_propBird_flyLoop" true)
  (`SkeletalMeshComponent.PlayAnimation` (`self.SkeletalMesh3`) "/Game/Characters/prop_bird/anim_propBird_flyLoop.anim_propBird_flyLoop" true)
  (`SkeletalMeshComponent.PlayAnimation` (`self.SkeletalMesh4`) "/Game/Characters/prop_bird/anim_propBird_flyLoop.anim_propBird_flyLoop" true)
  (`KismetSystemLibrary.Delay` 0.4)
  (`SkeletalMeshComponent.PlayAnimation` (`self.SkeletalMesh5`) "/Game/Characters/prop_bird/anim_propBird_flyLoop.anim_propBird_flyLoop" true)
  (`SkeletalMeshComponent.PlayAnimation` (`self.SkeletalMesh6`) "/Game/Characters/prop_bird/anim_propBird_flyLoop.anim_propBird_flyLoop" true)
  (`SkeletalMeshComponent.PlayAnimation` (`self.SkeletalMesh15`) "/Game/Characters/prop_bird/anim_propBird_flyLoop.anim_propBird_flyLoop" true)
  (`SkeletalMeshComponent.PlayAnimation` (`self.SkeletalMesh8`) "/Game/Characters/prop_bird/anim_propBird_flyLoop.anim_propBird_flyLoop" true)
  (`SkeletalMeshComponent.PlayAnimation` (`self.SkeletalMesh9`) "/Game/Characters/prop_bird/anim_propBird_flyLoop.anim_propBird_flyLoop" true)
  (`SkeletalMeshComponent.PlayAnimation` (`self.SkeletalMesh10`) "/Game/Characters/prop_bird/anim_propBird_flyLoop.anim_propBird_flyLoop" true)
  (`KismetSystemLibrary.Delay` 0.8)
  (`SkeletalMeshComponent.PlayAnimation` (`self.SkeletalMesh12`) "/Game/Characters/prop_bird/anim_propBird_flyLoop.anim_propBird_flyLoop" true)
  (`SkeletalMeshComponent.PlayAnimation` (`self.SkeletalMesh13`) "/Game/Characters/prop_bird/anim_propBird_flyLoop.anim_propBird_flyLoop" true)
  (`SkeletalMeshComponent.PlayAnimation` (`self.SkeletalMesh14`) "/Game/Characters/prop_bird/anim_propBird_flyLoop.anim_propBird_flyLoop" true)
  (`SkeletalMeshComponent.PlayAnimation` (`self.SkeletalMesh11`) "/Game/Characters/prop_bird/anim_propBird_flyLoop.anim_propBird_flyLoop" true)
  (`KismetSystemLibrary.Delay` 1.4))

(fn `UserConstructionScript`)