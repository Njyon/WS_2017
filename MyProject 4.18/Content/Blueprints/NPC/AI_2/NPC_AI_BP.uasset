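; NPC AI controller that runs a behavior tree and reacts to seeing the player.
; BeginPlay sets up the blackboard and tree; unpossessing sets the flag to stop AI logic.
; Perception focuses on a "Player"-tagged actor and writes it to the blackboard once per sighting, guarded by a flag.
; Losing sight only resets that flag; focus clearing, suspicion and enemy-key updates are unwired.
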(event `self.OnUnpossess`
  (params (UnpossessedPawn :type "Pawn Object Reference"))
  ;[1 1 1] If Ower is Dead stop Logic
  (set `self.bStopAILogicOnUnposses` true))

(event `self.ReceiveBeginPlay`
  ;[1 1 1] Select Blackboard and Run Behavior Tree
  (bind _blackboardcomponent (`self.UseBlackboard` "/Game/Blueprints/NPC/AI_2/AIBlackBoard.AIBlackBoard"))
  (`self.RunBehaviorTree` "/Game/Blueprints/NPC/AI_2/AILogic.AILogic")
  ;[1 1 1] Set Blackboard as a variable
  (set `self.BlackBoardComp` _blackboardcomponent))

(event `self.AIPerception.OnTargetPerceptionUpdated`
  (params (Actor :type "Actor Object Reference") (Stimulus :type "AIStimulus Structure"))
  (bind _returnvalue (`self.ActorHasTag` Actor "Player"))
  ;[1 1 1] AI 2.0 Perseption
  (if (`.bSuccessfullySensed` (break `AIStimulus` Stimulus))
    ;;[0.4409 1 0.2645] Set the Focus Point for the AI
    (if _returnvalue
      (if (not (`self.hasSetFocusPoint`))
        (`|ExecutionSequence`
          (:`then_0`
            (`self.K2_SetFocus` Actor)
            (set `self.hasSetFocusPoint` true))
          (:`then_1`
            (`BlackboardComponent.SetValueAsObject` (`self.BlackBoardComp`) "Player" Actor)))))
    (elif _returnvalue
      (set `self.hasSetFocusPoint` false))))

(fn `UpdateBlackboardEnemyKey`
  (params (ObjectValue :type "Object Object Reference") (self2 :type "Actor Object Reference") (AIStimulus :type "AIStimulus Structure (by ref)"))
  (bind _enemykey (`self.EnemyKey`))
  (bind _blackboardcomp (`self.BlackBoardComp`))
  (if (`self.ActorHasTag` self2 "Enemy")
    _
    (elif (`.bSuccessfullySensed` (break `AIStimulus` AIStimulus))
      (`BlackboardComponent.SetValueAsObject` _blackboardcomp _enemykey ObjectValue)
      (else
        (`BlackboardComponent.ClearValue` _blackboardcomp _enemykey)))))

(fn `UserConstructionScript`)