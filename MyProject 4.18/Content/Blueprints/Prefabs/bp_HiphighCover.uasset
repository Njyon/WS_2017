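; Hip-high cover prefab that vaults the first-person player across it along a spline when they overlap its box with CanSprint set.
; It snaps a spline end to the player based on distance, aligns the points sideways, then plays the JumpOver timeline forward or reversed to move them.
; A CamTilt timeline briefly rolls the view, and the spline resets afterward.
; The construction script places three meshes at the spline points.
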(event `self.Box.OnComponentBeginOverlap`
  (params (OverlappedComponent :type "PrimitiveComponent Object Reference") (OtherActor :type "Actor Object Reference") (OtherComp :type "PrimitiveComponent Object Reference") (OtherBodyIndex :type Integer) (bFromSweep :type Boolean) (SweepResult :type "HitResult Structure (by ref)"))
  (bind _spline (`self.Spline`))
  (bind _spline_2 (`self.Spline`))
  (bind _spline_3 (`self.Spline`))
  (bind _spline_4 (`self.Spline`))
  (bind _character_ref (`self.Character Ref`))
  (bind _spline_5 (`self.Spline`))
  (bind _spline_6 (`self.Spline`))
  (bind _character_ref_2 (`self.Character Ref`))
  (bind _returnvalue (`SplineComponent.GetNumberOfSplinePoints` (`self.Spline`)))
  (bind _returnvalue_location (`KismetMathLibrary.BreakTransform` (`self.GetTransform` (`self.Character Ref`))))
  (bind _returnvalue_2 (`SplineComponent.GetNumberOfSplinePoints` (`self.Spline`)))
  (bind _returnvalue_location_2 (`KismetMathLibrary.BreakTransform` (`self.GetTransform` (`self.Character Ref`))))
  (bind (_returnvalue_location_3 _returnvalue_rotation) (`KismetMathLibrary.BreakTransform` (`SceneComponent.GetRelativeTransform` (`Actor.RootComponent` (`self.Character Ref`)))))
  (bind _array (`|MakeArray` _returnvalue_2))
  (bind _array_2 (`|MakeArray` _returnvalue))
  (bind _output (`|GetArrayItem` _array_2))
  (bind _output_2 (`|GetArrayItem` _array_2 _returnvalue))
  (bind _returnvalue_3 (- _output 1))
  (bind _y (.y (`SplineComponent.GetLocationAtSplinePoint` _spline_2 _output "Local")))
  (bind _y_2 (.y (`SplineComponent.GetLocationAtSplinePoint` _spline_2 _output_2 "Local")))
  (if (== _character_ref OtherActor)
    (if (and (`self.canJumoOver`) (`MyProjectCharacter.canSprint` _character_ref))
      (set `self.canJumoOver` false)
      (`MyProjectCharacter.RevertedSlideCam` (`self.Character Ref`))
      (if (> (`KismetMathLibrary.VSize` (- (`SplineComponent.GetLocationAtSplinePoint` _spline_5 _returnvalue_3 "World") _returnvalue_location)) (`KismetMathLibrary.VSize` (- (`SplineComponent.GetLocationAtSplinePoint` _spline_5 _output_2 "World") _returnvalue_location)))
        ;[1 1 1] Snap First or Last Point to Player
        (`SplineComponent.SetLocationAtSplinePoint` _spline _output_2 _returnvalue_location_2 "World" true)
        (`|ExecutionSequence`
          (:`then_0`
            ;[1 1 1] Set New Position off the Spline
            (`SplineComponent.SetLocationAtSplinePoint` _spline_2 0 (`KismetMathLibrary.MakeVector` (.x (`SplineComponent.GetLocationAtSplinePoint` _spline_2 0 "Local")) _y_2 (.z (`SplineComponent.GetLocationAtSplinePoint` _spline_2 0 "Local"))) "Local" true))
          (:`then_1`
            (`SplineComponent.SetLocationAtSplinePoint` _spline_2 1 (`KismetMathLibrary.MakeVector` (.x (`SplineComponent.GetLocationAtSplinePoint` _spline_2 1 "Local")) _y_2 (.z (`SplineComponent.GetLocationAtSplinePoint` _spline_2 1 "Local"))) "Local" true))
          (:`then_2`
            (`SplineComponent.SetLocationAtSplinePoint` _spline_2 2 (`KismetMathLibrary.MakeVector` (.x (`SplineComponent.GetLocationAtSplinePoint` _spline_2 2 "Local")) _y_2 (.z (`SplineComponent.GetLocationAtSplinePoint` _spline_2 2 "Local"))) "Local" true))
          (:`then_3`
            ;[1 1 1] Snap First or Last Point to Player
            (`SplineComponent.SetLocationAtSplinePoint` _spline_4 _output_2 _returnvalue_location_2 "World" true)
            (`|ExecutionSequence`
              (:`then_0`
                ;[1 1 1] Cam Tilt
                (`/Engine/EditorBlueprintResources/StandardMacros.DoOnce` false :!label _label
                  (:`Completed`
                    (bind (_direction _tilt) (`Timeline|Cam Tilt` :!label _label_2)
                      (:`Update`
                        (`Controller.SetControlRotation` (`GameplayStatics.GetPlayerController` 0) (`KismetMathLibrary.RLerp` _returnvalue_rotation (`KismetMathLibrary.MakeRotator` -45.0 (.pitch _returnvalue_rotation) (.yaw _returnvalue_rotation)) _tilt)))))))
              (:`then_1`
                ;[1 1 1] Move Character Along Spline
                (bind (_direction_2 _movement) (`Timeline|JumpOver` :!via `PlayFromStart` :!label _label_3)
                  (:`Update`
                    (`self.K2_SetActorLocation` _character_ref_2 (`SplineComponent.GetLocationAtDistanceAlongSpline` _spline_6 (* (`SplineComponent.GetSplineLength` _spline_6) _movement) "World") true false))
                  (:`Finished`
                    (`MyProjectCharacter.SlideCam` _character_ref_2)
                    (`SplineComponent.SetLocationAtSplinePoint` _spline_3 (- (`|GetArrayItem` _array) 1) (`self.StartSplinePoint`) "World" true)
                    (`SplineComponent.SetLocationAtSplinePoint` _spline_3 (`|GetArrayItem` _array _returnvalue_2) (`self.EndSplinePoint`) "World" true)
                    (`SceneComponent.K2_SetRelativeTransform` (`self.Spline`) (`self.StartTransform`) false false)
                    (`KismetSystemLibrary.Delay` 0.2)
                    (set `self.canJumoOver` true))))
              (:`then_2`
                (`KismetSystemLibrary.Delay` 0.25)
                (`self.ReverseCam` :!label _label_4)))))
        (else
          (`SplineComponent.SetLocationAtSplinePoint` _spline _returnvalue_3 _returnvalue_location_2 "World" true)
          (`|ExecutionSequence`
            (:`then_0`
              (`SplineComponent.SetLocationAtSplinePoint` _spline_2 0 (`KismetMathLibrary.MakeVector` (.x (`SplineComponent.GetLocationAtSplinePoint` _spline_2 0 "Local")) _y (.z (`SplineComponent.GetLocationAtSplinePoint` _spline_2 0 "Local"))) "Local" true))
            (:`then_1`
              (`SplineComponent.SetLocationAtSplinePoint` _spline_2 1 (`KismetMathLibrary.MakeVector` (.x (`SplineComponent.GetLocationAtSplinePoint` _spline_2 1 "Local")) _y (.z (`SplineComponent.GetLocationAtSplinePoint` _spline_2 1 "Local"))) "Local" true))
            (:`then_2`
              (`SplineComponent.SetLocationAtSplinePoint` _spline_2 2 (`KismetMathLibrary.MakeVector` (.x (`SplineComponent.GetLocationAtSplinePoint` _spline_2 2 "Local")) _y (.z (`SplineComponent.GetLocationAtSplinePoint` _spline_2 2 "Local"))) "Local" true))
            (:`then_3`
              (`SplineComponent.SetLocationAtSplinePoint` _spline_4 _returnvalue_3 _returnvalue_location_2 "World" true)
              (`|ExecutionSequence`
                (:`then_0`
                  (goto _label))
                (:`then_1`
                  (goto _label_3 :!via `ReverseFromEnd`))
                (:`then_2`
                  (`KismetSystemLibrary.Delay` 0.25)
                  (goto _label_4))))))))))

(event `Key|E`
  (params (Key :type "Key Structure")))

(event `self.ReceiveBeginPlay`
  (bind _spline (`self.Spline`))
  (bind _returnvalue (`SplineComponent.GetNumberOfSplinePoints` (`self.Spline`)))
  (bind _array (`|MakeArray` _returnvalue))
  ;[1 1 1] Get Player and Enable Input
  (bind _asfirst_person_character (cast `/Game/Blueprints/Player/Behaviour/FirstPersonCharacter` (`GameplayStatics.GetPlayerCharacter` 0)))
  (set `self.Character Ref` _asfirst_person_character)
  (`self.EnableInput` (`GameplayStatics.GetPlayerController` 0))
  (`TimelineComponent.SetPlayRate` (`self.Cam Tilt`) 2.0)
  (`TimelineComponent.SetPlayRate` (`self.JumpOver`) 3.0)
  (set `self.StartSplinePoint` (`SplineComponent.GetLocationAtSplinePoint` _spline (`|GetArrayItem` _array) "World"))
  (set `self.EndSplinePoint` (`SplineComponent.GetLocationAtSplinePoint` _spline (`|GetArrayItem` _array _returnvalue) "World"))
  (set `self.StartTransform` (`SceneComponent.GetRelativeTransform` (`self.Spline`))))

(event `ReverseCam`
  (`|ExecutionSequence`
    (:`then_0`
      (goto _label :!via `Reset`))
    (:`then_1`
      (goto _label_2 :!via `Reverse`))))

(event `Key|T`
  (params (Key :type "Key Structure")))

(fn `UserConstructionScript`
  (bind _spline (`self.Spline`))
  (`SceneComponent.K2_SetRelativeTransform` (`self.StaticMesh`) (`KismetMathLibrary.MakeTransform` (`SplineComponent.GetLocationAndTangentAtSplinePoint` _spline 0 "Local")) true true)
  (`SceneComponent.K2_SetRelativeTransform` (`self.StaticMesh1`) (`KismetMathLibrary.MakeTransform` (`SplineComponent.GetLocationAndTangentAtSplinePoint` _spline 1 "Local")) true true)
  (`SceneComponent.K2_SetRelativeTransform` (`self.StaticMesh2`) (`KismetMathLibrary.MakeTransform` (`SplineComponent.GetLocationAndTangentAtSplinePoint` _spline 2 "Local")) true true))