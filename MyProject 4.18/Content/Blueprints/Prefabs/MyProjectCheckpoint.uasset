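; Checkpoint prefab actor that shows a highlight for the active checkpoint and plays feedback when it is reached.
; On BeginPlay the highlight mesh is hidden unless this is the first checkpoint, and ActivateNextCP reveals it later.
; OnCheckpoint raises the checkpoint material's visibility parameter, recolors the highlight via a dynamic material instance, and activates the PAUTrapTarget and PCheckpoint components.
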(event `self.ReceiveBeginPlay`
  (if (not (`self.firstCP`))
    (`SceneComponent.SetVisibility` (`self.mesh_checkpointHighlight`) false false)))

(event `self.ActivateNextCP`
  (`SceneComponent.SetVisibility` (`self.mesh_checkpointHighlight`) true false))

(event `self.OnCheckpoint`
  (`MeshComponent.SetScalarParameterValueOnMaterials` (`self.mesh_checkpoint`) "Visibility" 1.0)
  (bind _returnvalue (`PrimitiveComponent.CreateDynamicMaterialInstance` (`self.mesh_checkpointHighlight`) 0 null))
  (`MaterialInstanceDynamic.SetVectorParameterValue` _returnvalue "ColorCheckpoint" (struct :`R` 2.2 :`G` 1.6 :`B` 0.4 :`A` 1.0))
  (`ActorComponent.Activate` (`self.P_AU_Trap_Target`) false)
  (`ActorComponent.Activate` (`self.P_checkpoint`) false))

(fn `UserConstructionScript`)