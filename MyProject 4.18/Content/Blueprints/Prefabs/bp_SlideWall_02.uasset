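; Slide-wall prefab that carries the first-person player along a spline when they enter its box while able to sprint or already sliding.
; On overlap it moves the nearer spline end to the player, then plays the Slide timeline forward or in reverse to set the character's location along the spline.
; When finished it calls the character's slide camera, restores the saved endpoints and re-arms after a short delay.
; Disconnected lerp timelines and debug prints remain in the graph.
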(event `self.ReceiveBeginPlay`
  (bind _spline (`self.Spline`))
  (bind _returnvalue (`SplineComponent.GetNumberOfSplinePoints` (`self.Spline`)))
  (bind _array (`|MakeArray` _returnvalue))
  ;[1 1 1] Get Player
  (bind _asfirst_person_character (cast `/Game/Blueprints/Player/Behaviour/FirstPersonCharacter` (`GameplayStatics.GetPlayerCharacter` 0)))
  (set `self.CharacterRef` _asfirst_person_character)
  (`self.EnableInput` (`GameplayStatics.GetPlayerController` 0))
  (`TimelineComponent.SetPlayRate` (`self.Slide`) 2.0)
  (set `self.splineStartPoint` (`SplineComponent.GetLocationAtSplinePoint` _spline (`|GetArrayItem` _array) "World"))
  (set `self.splineEndPoint` (`SplineComponent.GetLocationAtSplinePoint` _spline (`|GetArrayItem` _array _returnvalue) "World")))

(event `Key|E`
  (params (Key :type "Key Structure")))

(event `self.Box.OnComponentBeginOverlap`
  (params (OverlappedComponent :type "PrimitiveComponent Object Reference") (OtherActor :type "Actor Object Reference") (OtherComp :type "PrimitiveComponent Object Reference") (OtherBodyIndex :type Integer) (bFromSweep :type Boolean) (SweepResult :type "HitResult Structure (by ref)"))
  (bind _spline (`self.Spline`))
  (bind _spline_2 (`self.Spline`))
  (bind _spline_3 (`self.Spline`))
  (bind _characterref (`self.CharacterRef`))
  (bind _spline_4 (`self.Spline`))
  (bind _characterref_2 (`self.CharacterRef`))
  (bind _returnvalue (`SplineComponent.GetNumberOfSplinePoints` _spline_2))
  (bind _returnvalue_2 (`SplineComponent.GetNumberOfSplinePoints` (`self.Spline`)))
  (bind _returnvalue_location (`KismetMathLibrary.BreakTransform` (`self.GetTransform` (`self.CharacterRef`))))
  (bind _returnvalue_location_2 (`KismetMathLibrary.BreakTransform` (`self.GetTransform` (`self.CharacterRef`))))
  (bind _array (`|MakeArray` _returnvalue_2))
  (bind _array_2 (`|MakeArray` _returnvalue))
  (bind _output (`|GetArrayItem` _array_2))
  (bind _output_2 (`|GetArrayItem` _array_2 _returnvalue))
  (bind _returnvalue_3 (- _output 1))
  (if (and (== _characterref OtherActor) (`self.canSlide`))
    (set `self.canSlide` false)
    (if (or (`MyProjectCharacter.canSprint` _characterref) (`MyProjectCharacter.sliding` _characterref))
      (`MyProjectCharacter.RevertedSlideCam` _characterref)
      (if (> (`KismetMathLibrary.VSize` (- (`SplineComponent.GetLocationAtSplinePoint` _spline_4 _output "World") _returnvalue_location)) (`KismetMathLibrary.VSize` (- (`SplineComponent.GetLocationAtSplinePoint` _spline_4 _output_2 "World") _returnvalue_location)))
        (`SplineComponent.SetLocationAtSplinePoint` _spline_3 _output_2 _returnvalue_location_2 "World" true)
        (`KismetSystemLibrary.PrintString` (`KismetStringLibrary.Conv_IntToString` _output_2))
        ;[1 1 1] Move Along Spline
        (bind (_direction _movement) (`Timeline|Slide` :`NewTime` 0.2 :!via `PlayFromStart` :!label _label)
          (:`Update`
            (`self.K2_SetActorLocation` _characterref_2 (`SplineComponent.GetLocationAtDistanceAlongSpline` _spline_2 (* (`SplineComponent.GetSplineLength` _spline_2) _movement) "World") true false))
          (:`Finished`
            (`MyProjectCharacter.SlideCam` _characterref_2)
            (`SplineComponent.SetLocationAtSplinePoint` _spline (- (`|GetArrayItem` _array) 1) (`self.splineStartPoint`) "World" true)
            (`SplineComponent.SetLocationAtSplinePoint` _spline (`|GetArrayItem` _array _returnvalue_2) (`self.splineEndPoint`) "World" true)
            (`KismetSystemLibrary.Delay` 0.2)
            (set `self.canSlide` true)))
        (else
          (`SplineComponent.SetLocationAtSplinePoint` _spline_3 _returnvalue_3 _returnvalue_location_2 "World" true)
          (`KismetSystemLibrary.PrintString` (`KismetStringLibrary.Conv_IntToString` _returnvalue_3))
          (goto _label :!via `ReverseFromEnd`))))))

(event `self.Box.OnComponentEndOverlap`
  (params (OverlappedComponent :type "PrimitiveComponent Object Reference") (OtherActor :type "Actor Object Reference") (OtherComp :type "PrimitiveComponent Object Reference") (OtherBodyIndex :type Integer))
  (if (== OtherActor (`self.CharacterRef`))
    (set `self.canSlide` true)))

(fn `UserConstructionScript`)