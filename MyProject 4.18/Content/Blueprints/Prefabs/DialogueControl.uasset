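; DialogueControl is a trigger actor that fires dialogue-stage events on the FirstPersonCharacter when the character overlaps it.
; The Intro, Halfway, Almost and Outro booleans select which matching BP event it calls on the character.
; A Sequence checks each flag independently, and each branch has its own DoOnce, so each event fires only once per actor instance.
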(event `self.ReceiveActorBeginOverlap`
  (params (OtherActor :type "Actor Object Reference"))
  (bind _asfirst_person_character (cast `/Game/Blueprints/Player/Behaviour/FirstPersonCharacter` OtherActor))
  (`|ExecutionSequence`
    (:`then_0`
      (if (`self.Intro`)
        (`/Engine/EditorBlueprintResources/StandardMacros.DoOnce` false
          (:`Completed`
            (`MyProjectCharacter.OnIntroBPEvent` _asfirst_person_character)))))
    (:`then_1`
      (if (`self.Halfway`)
        (`/Engine/EditorBlueprintResources/StandardMacros.DoOnce` false
          (:`Completed`
            (`MyProjectCharacter.OnHalfwayBPEvent` _asfirst_person_character)))))
    (:`then_2`
      (if (`self.Almost`)
        (`/Engine/EditorBlueprintResources/StandardMacros.DoOnce` false
          (:`Completed`
            (`MyProjectCharacter.OnAlmostBPEvent` _asfirst_person_character)))))
    (:`then_3`
      (if (`self.Outro`)
        (`/Engine/EditorBlueprintResources/StandardMacros.DoOnce` false
          (:`Completed`
            (`MyProjectCharacter.OnOutroBPEvent` _asfirst_person_character)))))))

(fn `UserConstructionScript`)