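; Spline guide actor that shows a path of spline meshes while the player is in slow motion and hides it afterward.
; The construction script builds one spline mesh per segment of the Spline.
; BeginPlay gives each mesh a dynamic material and binds Show and Hide to FirstPersonCharacter's slomo events.
; These play or reverse the Alpha timeline, which ignores time dilation and drives the materials' TEST parameter.
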(event `self.ReceiveBeginPlay`
  (bind _asfirst_person_character (cast `/Game/Blueprints/Player/Behaviour/FirstPersonCharacter` (`GameplayStatics.GetPlayerCharacter` 0)))
  (add `/Game/Blueprints/Player/Behaviour/FirstPersonCharacter.inSlomo` _asfirst_person_character (delegate `Show`))
  (add `/Game/Blueprints/Player/Behaviour/FirstPersonCharacter.outSlomo` _asfirst_person_character (delegate `Hide`))
  (for _array_element (`self.meshes`)
    (bind _returnvalue (`PrimitiveComponent.CreateDynamicMaterialInstance` _array_element 0 "/Game/Temp/TESTSPLINE.TESTSPLINE"))
    (`KismetArrayLibrary.Array_Add` (`self.Materials`) _returnvalue)
    (`TimelineComponent.SetIgnoreTimeDilation` (`self.Alpha`) true)
    (for _array_element_2 (`self.Materials`)
      (`MaterialInstanceDynamic.SetScalarParameterValue` _array_element_2 "TEST" 0.0))))

(event `Hide`
  (bind (_direction _newtrack_1) (`Timeline|Alpha` :!via `Reverse` :!label _label)
    (:`Update`
      (for _array_element (`self.Materials`)
        (`MaterialInstanceDynamic.SetScalarParameterValue` _array_element "TEST" _newtrack_1)))))

(event `Show`
  (goto _label))

(fn `UserConstructionScript`
  (bind _spline (`self.Spline`))
  (for _index (range (+ (- (`SplineComponent.GetNumberOfSplinePoints` _spline) 2) 1))
    (bind _returnvalue (`AddComponent|NODE_AddSplineMeshComponent-0`))
    (`KismetArrayLibrary.Array_Add` (`self.meshes`) _returnvalue)
    (`SceneComponent.K2_AttachToComponent` _returnvalue (`self.DefaultSceneRoot`) "None" "KeepRelative" "KeepRelative" "KeepRelative" true)
    (bind (_location _tangent) (`SplineComponent.GetLocationAndTangentAtSplinePoint` _spline _index "Local"))
    (bind (_location_2 _tangent_2) (`SplineComponent.GetLocationAndTangentAtSplinePoint` _spline (+ _index 1) "Local"))
    (`SplineMeshComponent.SetStartAndEnd` _returnvalue _location _tangent _location_2 _tangent_2 true)))