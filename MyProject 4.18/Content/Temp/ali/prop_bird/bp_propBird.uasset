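; Prop bird flock actor made of many skeletal mesh components that loop a flying animation.
; BeginPlay starts the fly loop in three groups separated by short delays, so the birds flap out of sync.
; Tick applies a small constant +Y force to the root bone of five of the meshes only.
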(event `self.ReceiveTick`
  (params (DeltaSeconds :type "Float (single-precision)"))
  (`PrimitiveComponent.AddForce` (`self.Bird`) (0.0 1.0 0.0) "root" false)
  (`PrimitiveComponent.AddForce` (`self.SkeletalMesh7`) (0.0 1.0 0.0) "root" false)
  (`PrimitiveComponent.AddForce` (`self.SkeletalMesh`) (0.0 1.0 0.0) "root" false)
  (`PrimitiveComponent.AddForce` (`self.SkeletalMesh1`) (0.0 1.0 0.0) "root" false)
  (`PrimitiveComponent.AddForce` (`self.SkeletalMesh2`) (0.0 1.0 0.0) "root" false))

(event `self.ReceiveBeginPlay`
  (`SkeletalMeshComponent.PlayAnimation` (`self.Bird`) "/Game/Temp/ali/prop_bird/anim_propBird_flyLoop.anim_propBird_flyLoop" true)
  (`SkeletalMeshComponent.PlayAnimation` (`self.SkeletalMesh7`) "/Game/Temp/ali/prop_bird/anim_propBird_flyLoop.anim_propBird_flyLoop" true)
  (`SkeletalMeshComponent.PlayAnimation` (`self.SkeletalMesh`) "/Game/Temp/ali/prop_bird/anim_propBird_flyLoop.anim_propBird_flyLoop" true)
  (`SkeletalMeshComponent.PlayAnimation` (`self.SkeletalMesh1`) "/Game/Temp/ali/prop_bird/anim_propBird_flyLoop.anim_propBird_flyLoop" true)
  (`SkeletalMeshComponent.PlayAnimation` (`self.SkeletalMesh2`) "/Game/Temp/ali/prop_bird/anim_propBird_flyLoop.anim_propBird_flyLoop" true)
  (`SkeletalMeshComponent.PlayAnimation` (`self.SkeletalMesh3`) "/Game/Temp/ali/prop_bird/anim_propBird_flyLoop.anim_propBird_flyLoop" true)
  (`SkeletalMeshComponent.PlayAnimation` (`self.SkeletalMesh4`) "/Game/Temp/ali/prop_bird/anim_propBird_flyLoop.anim_propBird_flyLoop" true)
  (`KismetSystemLibrary.Delay` 0.4)
  (`SkeletalMeshComponent.PlayAnimation` (`self.SkeletalMesh5`) "/Game/Temp/ali/prop_bird/anim_propBird_flyLoop.anim_propBird_flyLoop" true)
  (`SkeletalMeshComponent.PlayAnimation` (`self.SkeletalMesh6`) "/Game/Temp/ali/prop_bird/anim_propBird_flyLoop.anim_propBird_flyLoop" true)
  (`SkeletalMeshComponent.PlayAnimation` (`self.SkeletalMesh15`) "/Game/Temp/ali/prop_bird/anim_propBird_flyLoop.anim_propBird_flyLoop" true)
  (`SkeletalMeshComponent.PlayAnimation` (`self.SkeletalMesh8`) "/Game/Temp/ali/prop_bird/anim_propBird_flyLoop.anim_propBird_flyLoop" true)
  (`SkeletalMeshComponent.PlayAnimation` (`self.SkeletalMesh9`) "/Game/Temp/ali/prop_bird/anim_propBird_flyLoop.anim_propBird_flyLoop" true)
  (`SkeletalMeshComponent.PlayAnimation` (`self.SkeletalMesh10`) "/Game/Temp/ali/prop_bird/anim_propBird_flyLoop.anim_propBird_flyLoop" true)
  (`KismetSystemLibrary.Delay` 0.8)
  (`SkeletalMeshComponent.PlayAnimation` (`self.SkeletalMesh12`) "/Game/Temp/ali/prop_bird/anim_propBird_flyLoop.anim_propBird_flyLoop" true)
  (`SkeletalMeshComponent.PlayAnimation` (`self.SkeletalMesh13`) "/Game/Temp/ali/prop_bird/anim_propBird_flyLoop.anim_propBird_flyLoop" true)
  (`SkeletalMeshComponent.PlayAnimation` (`self.SkeletalMesh14`) "/Game/Temp/ali/prop_bird/anim_propBird_flyLoop.anim_propBird_flyLoop" true)
  (`SkeletalMeshComponent.PlayAnimation` (`self.SkeletalMesh11`) "/Game/Temp/ali/prop_bird/anim_propBird_flyLoop.anim_propBird_flyLoop" true)
  (`KismetSystemLibrary.Delay` 1.4))

(fn `UserConstructionScript`)