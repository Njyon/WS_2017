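; Ladder actor that lets the first-person character climb while inside its Box trigger.
; Entering the box flags the character as on a ladder and calls its OnLadder handler.
; Leaving clears the ladder and flying flags and restores walking movement.
; On exit it also calls LadderClimbUp unless spacebar is held or the vertical axis is fully down.
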(event `self.Box.OnComponentBeginOverlap`
  (params (OverlappedComponent :type "PrimitiveComponent Object Reference") (OtherActor :type "Actor Object Reference") (OtherComp :type "PrimitiveComponent Object Reference") (OtherBodyIndex :type Integer) (bFromSweep :type Boolean) (SweepResult :type "HitResult Structure (by ref)"))
  (bind _asfirst_person_character (cast `/Game/Dynamic/Player/Behaviour/FirstPersonCharacter` OtherActor))
  (set `MyProjectCharacter.isOnLadder` true _asfirst_person_character)
  (`/Game/Dynamic/Player/Behaviour/FirstPersonCharacter.OnLadder` _asfirst_person_character))

(event `self.Box.OnComponentEndOverlap`
  (params (OverlappedComponent :type "PrimitiveComponent Object Reference") (OtherActor :type "Actor Object Reference") (OtherComp :type "PrimitiveComponent Object Reference") (OtherBodyIndex :type Integer))
  (bind _asfirst_person_character (cast `/Game/Dynamic/Player/Behaviour/FirstPersonCharacter` OtherActor))
  (set `MyProjectCharacter.isOnLadder` false _asfirst_person_character)
  (set `MyProjectCharacter.isFlying` false _asfirst_person_character)
  (`CharacterMovementComponent.SetMovementMode` (`Character.CharacterMovement` _asfirst_person_character) "MOVE_Walking" 0)
  (if (`MyProjectCharacter.isSpacebarPressed` _asfirst_person_character)
    _
    (elif (== (== (`/Game/Dynamic/Player/Behaviour/FirstPersonCharacter.VAxis` _asfirst_person_character) -1.0) false)
      (`/Game/Dynamic/Player/Behaviour/FirstPersonCharacter.LadderClimbUp` _asfirst_person_character))))

(fn `UserConstructionScript`)