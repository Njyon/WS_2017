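; Trigger volume that sends the first-person character sliding in the direction of its arrow component.
; On overlap it sets the Sliding flag, starts the slide camera, zeroes ground friction and braking, and launches the player along the arrow's forward vector.
; A second launch fires after a short delay, marked as an old fix.
; Leaving the area clears the flag, restores fixed friction and braking values, and reverses the camera effect.
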(event `self.SlideArea.OnComponentBeginOverlap`
  (params (OverlappedComponent :type "PrimitiveComponent Object Reference") (OtherActor :type "Actor Object Reference") (OtherComp :type "PrimitiveComponent Object Reference") (OtherBodyIndex :type Integer) (bFromSweep :type Boolean) (SweepResult :type "HitResult Structure (by ref)"))
  ;[1 1 1] Slide (Arrow direction)
  (bind _asfirst_person_character (cast `/Game/Dynamic/Player/Behaviour/FirstPersonCharacter` OtherActor))
  (set `/Game/Dynamic/Player/Behaviour/FirstPersonCharacter.sliding` true _asfirst_person_character)
  (`/Game/Dynamic/Player/Behaviour/FirstPersonCharacter.SlideCam` _asfirst_person_character)
  (bind _charactermovement (`Character.CharacterMovement` _asfirst_person_character))
  (set `CharacterMovementComponent.GroundFriction` 0.0 _charactermovement)
  (set `CharacterMovementComponent.BrakingDecelerationWalking` 0.0 _charactermovement)
  (set `CharacterMovementComponent.BrakingFrictionFactor` 0.0 _charactermovement)
  (`|ExecutionSequence`
    (:`then_0`
      _)
    (:`then_1`
      ;;[1 0 0.06152] Gammel FIX
      (`KismetSystemLibrary.Delay` 0.2)))
  (`Character.LaunchCharacter` _asfirst_person_character (* (`SceneComponent.GetForwardVector` (`self.Arrow`)) 1000.0) true false))

(event `self.SlideArea.OnComponentEndOverlap`
  (params (OverlappedComponent :type "PrimitiveComponent Object Reference") (OtherActor :type "Actor Object Reference") (OtherComp :type "PrimitiveComponent Object Reference") (OtherBodyIndex :type Integer))
  ;[1 1 1] Stop Sliding
  (bind _asfirst_person_character (cast `/Game/Dynamic/Player/Behaviour/FirstPersonCharacter` OtherActor))
  (set `/Game/Dynamic/Player/Behaviour/FirstPersonCharacter.sliding` false _asfirst_person_character)
  (bind _charactermovement (`Character.CharacterMovement` _asfirst_person_character))
  (set `CharacterMovementComponent.GroundFriction` 8.0 _charactermovement)
  (set `CharacterMovementComponent.BrakingDecelerationWalking` 2048.0 _charactermovement)
  (set `CharacterMovementComponent.BrakingFrictionFactor` 2.0 _charactermovement)
  (`/Game/Dynamic/Player/Behaviour/FirstPersonCharacter.ReveredSlideCam` _asfirst_person_character))

(fn `UserConstructionScript`)