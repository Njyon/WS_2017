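; AI controller for guard NPCs that starts their behavior tree and reports perceived targets to it.
; BeginPlay sets up the Patrol_Data blackboard, runs Guard_BT and caches the blackboard component.
; Perception updates ignore actors tagged Enemy, setting the enemy key and isSuspicious on sensing, and clearing only the key on loss.
; On unpossess, it sets the flag to stop AI logic.
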(event `self.OnUnpossess`
  (params (UnpossessedPawn :type "Pawn Object Reference"))
  ;[1 1 1] If Ower is Dead stop Logic
  (set `self.bStopAILogicOnUnposses` true))

(event `self.ReceiveBeginPlay`
  ;[1 1 1] Select Blackboard and Run Behavior Tree
  (bind _blackboardcomponent (`self.UseBlackboard` "/Game/Blueprints/NPC/AI/Patrol_Data.Patrol_Data"))
  (`self.RunBehaviorTree` "/Game/Blueprints/NPC/AI/Guard_BT.Guard_BT")
  ;[1 1 1] Set Blackboard as a variable
  (set `self.BlackBoardComp` _blackboardcomponent))

(event `self.AIPerception.OnTargetPerceptionUpdated`
  (params (Actor :type "Actor Object Reference") (Stimulus :type "AIStimulus Structure"))
  ;[1 1 1] Sees player / Yes-No
  (`|ExecutionSequence`
    (:`then_0`
      (`self.UpdateBlackboardEnemyKey` Actor Actor Stimulus))
    (:`then_1`
      (if (`self.ActorHasTag` Actor "Enemy")
        _
        (elif (`.bSuccessfullySensed` (break `AIStimulus` Stimulus))
          (`BlackboardComponent.SetValueAsBool` (`AIBlueprintHelperLibrary.GetBlackboard` null) "isSuspicious" true))))))

(fn `UpdateBlackboardEnemyKey`
  (params (ObjectValue :type "Object Object Reference") (self2 :type "Actor Object Reference") (AIStimulus :type "AIStimulus Structure (by ref)"))
  (bind _enemykey (`self.EnemyKey`))
  (bind _blackboardcomp (`self.BlackBoardComp`))
  (if (`self.ActorHasTag` self2 "Enemy")
    _
    (elif (`.bSuccessfullySensed` (break `AIStimulus` AIStimulus))
      (`BlackboardComponent.SetValueAsObject` _blackboardcomp _enemykey ObjectValue)
      (else
        (`BlackboardComponent.ClearValue` _blackboardcomp _enemykey)))))

(fn `UserConstructionScript`)